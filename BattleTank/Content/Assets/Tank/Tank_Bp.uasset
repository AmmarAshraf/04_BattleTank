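; Tank Blueprint that handles player camera aiming and fire input.
; Aim axes rotate the azimuth gimbal in yaw and the spring arm in pitch, scaled by frame time.
; The Fire action calls Fire, which is not defined in these graphs.
; The construction script passes the Barrel and Turret components to the aiming setters, keeping this Blueprint to input and component wiring.
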(event Input|ActionEvents|InputActionFire
  (params (Key :type Key%20Structure))
  (:Pressed
    (Class|Tank|Fire)))

(event Input|AxisEvents|InputAxisAim_Azimuth
  (params (AxisValue :type Float%20%28single-precision%29))
  ;[1 1 1] Axis binding
  (Transformation|AddLocalRotation (Variables|Components|GetAzamuthGimbal) (Math|Rotator|MakeRotator 0.0 0.0 (* AxisValue (Utilities|Time|GetWorldDeltaSeconds) 1e+02)) false false))

(event Input|AxisEvents|InputAxisAim_Elevation
  (params (AxisValue :type Float%20%28single-precision%29))
  ;[1 1 1] Axis binding
  (Transformation|AddLocalRotation (Variables|Components|GetSpringArm) (Math|Rotator|MakeRotator 0.0 (* AxisValue (Utilities|Time|GetWorldDeltaSeconds) 1e+02) 0.0) false false))

(fn ConstructionScript
  (Utilities|FlowControl|Sequence
    (:then_0
      (Class|Tank|SetAimingBarrelComponenet (Variables|Components|GetBarrel)))
    (:then_1
      (Class|Tank|SetAimingTurretComponenet (Variables|Components|GetTurret)))))